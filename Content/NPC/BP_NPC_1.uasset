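; Talkable NPC Blueprint that shows an interaction prompt and plays a linear dialogue.
; Each Talk call creates or advances the WB_Dialogue widget through the Dialogue array with a sound per line, then closes and resets after the last.
; PromptTrigger overlaps toggle the prompt, with a DoOnce that hides it again almost immediately on first overlap.
; Leaving the trigger resets the conversation and removes the widget.
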(event `/Game/NPC/BPI_Dialogue.Talk`
  (if (`self.IsTalk`)
    (if (< (`self.Talk_Index`) (`KismetArrayLibrary.Array_Length` (`self.Dialogue`)))
      (`TextBlock.SetText` (`/Game/NPC/WB_Dialogue.TalkText` (`self.UI`)) (`KismetTextLibrary.Conv_StringToText` (`|GetArrayItem` (`self.Dialogue`) (`self.Talk_Index`))) :!label _label)
      (`/Engine/EditorBlueprintResources/StandardMacros.IncrementInt` (`self.Talk_Index`)
        (:`  `
          (`GameplayStatics.PlaySound2D` "/Game/GameContent/SFX/AssetPack/Footstep/WAV/Footstep_Concrete_Type_01_01.Footstep_Concrete_Type_01_01" 1.0 1.0 0.0 null null)))
      (else
        (`Widget.RemoveFromParent` (`self.UI`))
        (set `self.Talk_Index` 0)
        (set `self.IsTalk` false)))
    (else
      (set `self.IsTalk` true)
      (bind _returnvalue (`|CreateWidget` "/Game/NPC/WB_Dialogue.WB_Dialogue_C" (`GameplayStatics.GetPlayerController` 0)))
      (bind _output_get (set `self.UI` _returnvalue))
      (`UserWidget.AddToViewport` _output_get 0)
      (goto _label))))

(event `self.PromptTrigger.OnComponentBeginOverlap`
  (params (OverlappedComponent :type "PrimitiveComponent Object Reference") (OtherActor :type "Actor Object Reference") (OtherComp :type "PrimitiveComponent Object Reference") (OtherBodyIndex :type Integer) (bFromSweep :type Boolean) (SweepResult :type "HitResult Structure (by ref)"))
  (bind _interactprompt (`self.InteractPrompt`))
  (`SceneComponent.SetVisibility` _interactprompt true false)
  (`/Engine/EditorBlueprintResources/StandardMacros.DoOnce` false
    (:`Completed`
      (`KismetSystemLibrary.Delay` 0.01)
      (`SceneComponent.SetVisibility` _interactprompt false false))))

(event `self.PromptTrigger.OnComponentEndOverlap`
  (params (OverlappedComponent :type "PrimitiveComponent Object Reference") (OtherActor :type "Actor Object Reference") (OtherComp :type "PrimitiveComponent Object Reference") (OtherBodyIndex :type Integer))
  (`SceneComponent.SetVisibility` (`self.InteractPrompt`) false false)
  (set `self.Talk_Index` 0)
  (set `self.IsTalk` false)
  (`/Engine/EditorBlueprintResources/StandardMacros.IsValid` (`self.UI`)
    (:`Is Valid`
      (`Widget.RemoveFromParent` (`self.UI`)))))

(fn `UserConstructionScript`)