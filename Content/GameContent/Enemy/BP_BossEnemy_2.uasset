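; BP_BossEnemy_2 is a boss enemy Blueprint that adds an on-screen health bar to its parent class.
; It creates a WB_BossHealth widget on BeginPlay and sets the bar to Health over MaxHealth every tick.
; Seeing a pawn through PawnSensing calls SpotPlayer and adds the widget to the viewport once.
; Death sets a Dead flag, guarded to run once, and removes the widget.
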(event `self.ReceiveBeginPlay`
  (`parent.ReceiveBeginPlay`)
  (bind _returnvalue (`|CreateWidget` "/Game/GameContent/Widgets/WB_BossHealth.WB_BossHealth_C" (`GameplayStatics.GetPlayerController` 0)))
  (set `self.BossHealth` _returnvalue))

(event `self.ReceiveTick`
  (params (DeltaSeconds :type "Float (single-precision)"))
  (`parent.ReceiveTick` DeltaSeconds)
  (`ProgressBar.SetPercent` (`/Game/GameContent/Widgets/WB_BossHealth.HealthBar` (`self.BossHealth`)) (/ (`self.Health`) (`self.Max Health`))))

(event `self.PawnSensing.OnSeePawn`
  (params (Pawn :type "Pawn Object Reference"))
  (`self.SpotPlayer`)
  (`/Engine/EditorBlueprintResources/StandardMacros.DoOnce` false
    (:`Completed`
      (`UserWidget.AddToViewport` (`self.BossHealth`) 0))))

(event `self.Death`
  (if (not (`self.Dead`))
    (set `self.Dead` true)
    (`Widget.RemoveFromParent` (`self.BossHealth`))))

(fn `UserConstructionScript`
  (`parent.UserConstructionScript`))