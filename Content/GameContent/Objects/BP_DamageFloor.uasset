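; BP_DamageFloor is a hazard floor, treated as spikes, that repeatedly damages the player standing in its Box volume.
; Box overlap events set the IsInSpikes flag and store the entering actor as PlayerRef, without filtering by class.
; Tick runs through a short Delay to throttle damage, then casts PlayerRef to BP_Player and calls HitReact with fixed damage while the flag is set.
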(event `self.ReceiveBeginPlay`
  (set `self.IsInSpikes` false))

(event `self.ReceiveTick`
  (params (DeltaSeconds :type "Float (single-precision)"))
  (`KismetSystemLibrary.Delay` 0.4)
  (if (`self.IsInSpikes`)
    (bind _asbp_player (cast `/Game/GameContent/Mannequin/BP_Player` (`self.PlayerRef`)))
    (`/Game/GameContent/Mannequin/BP_Mannequin.Hit React` _asbp_player _asbp_player 2.0)))

(event `self.Box.OnComponentBeginOverlap`
  (params (OverlappedComponent :type "PrimitiveComponent Object Reference") (OtherActor :type "Actor Object Reference") (OtherComp :type "PrimitiveComponent Object Reference") (OtherBodyIndex :type Integer) (bFromSweep :type Boolean) (SweepResult :type "HitResult Structure (by ref)"))
  (set `self.IsInSpikes` true)
  (set `self.PlayerRef` OtherActor))

(event `self.Box.OnComponentEndOverlap`
  (params (OverlappedComponent :type "PrimitiveComponent Object Reference") (OtherActor :type "Actor Object Reference") (OtherComp :type "PrimitiveComponent Object Reference") (OtherBodyIndex :type Integer))
  (set `self.IsInSpikes` false))

(fn `UserConstructionScript`)