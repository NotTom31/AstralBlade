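; BP_Blackhole is a black hole environment VFX actor built from accretion disc, event horizon glow, and top and bottom accretion sphere meshes.
; Its construction script creates a dynamic material instance on each mesh and applies a shared Color to all four.
; The disc's DepthFade is multiplied by the length of the root's world scale vector so it follows actor size.
; The event graph holds only disabled stubs, so no gameplay logic runs.
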(fn `UserConstructionScript`
  (bind _returnvalue (`PrimitiveComponent.CreateDynamicMaterialInstance` (`self.SM_AccrectionDisc`) 0 null "None"))
  (`MaterialInstanceDynamic.SetScalarParameterValue` _returnvalue "DepthFade" (* (`self.Accretion Disc Depth Fade`) (`KismetMathLibrary.VSize` (`SceneComponent.K2_GetComponentScale` (`self.DefaultSceneRoot`)))))
  (`MaterialInstanceDynamic.SetVectorParameterValue` _returnvalue "Color" (`self.Color`))
  (bind _returnvalue_2 (`PrimitiveComponent.CreateDynamicMaterialInstance` (`self.SM_EventHorizonGlow`) 0 null "None"))
  (`MaterialInstanceDynamic.SetVectorParameterValue` _returnvalue_2 "Color" (`self.Color`))
  (bind _returnvalue_3 (`PrimitiveComponent.CreateDynamicMaterialInstance` (`self.SM_VFX_AccretionSphereTop`) 0 null "None"))
  (`MaterialInstanceDynamic.SetVectorParameterValue` _returnvalue_3 "Color" (`self.Color`))
  (bind _returnvalue_4 (`PrimitiveComponent.CreateDynamicMaterialInstance` (`self.SM_VFX_AccretionSphereBottom`) 0 null "None"))
  (`MaterialInstanceDynamic.SetVectorParameterValue` _returnvalue_4 "Color" (`self.Color`)))